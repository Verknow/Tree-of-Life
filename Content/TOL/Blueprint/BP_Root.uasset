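; BP_Root is a placeable root actor in the 2D game that tracks how many roots exist.
; On BeginPlay it increments the root count on GM_2DGame, and on Destroyed it decrements it.
; Placement also triggers a brief RootBurst particle effect, switched off after a short delay, and plays a 2D placing sound.
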(event `self.ReceiveBeginPlay`
  (`/Engine/EditorBlueprintResources/StandardMacros.IncrementInt` (`/Game/TOL/Blueprint/GM_2DGame.No.Roots` (cast `/Game/TOL/Blueprint/GM_2DGame` (`GameplayStatics.GetGameMode`) :!pure true))
    (:`  `
      (`|ExecutionSequence`
        (:`then_0`
          ;[1 1 1] Particle system
          (`ActorComponent.Activate` (`self.RootBurst`) false)
          (`KismetSystemLibrary.Delay` 0.2)
          (`ActorComponent.Deactivate` (`self.RootBurst`)))
        (:`then_1`
          (`GameplayStatics.PlaySound2D` "/Game/TOL/Audio/PlacingSound1.PlacingSound1"))))))

(event `self.ReceiveDestroyed`
  (`/Engine/EditorBlueprintResources/StandardMacros.DecrementInt` (`/Game/TOL/Blueprint/GM_2DGame.No.Roots` (cast `/Game/TOL/Blueprint/GM_2DGame` (`GameplayStatics.GetGameMode`) :!pure true))))

(fn `UserConstructionScript`)