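; Game mode for a 2D tree-growing game that runs the tree's water, sunlight and nutrient economy.
; BeginPlay adds the resource bar, tutorial, feedback and main menu widgets, starts music, and pauses with pawn input disabled.
; Tick scales resource changes by a multiplier and delta time: roots supply water and nutrients, leaves consume water and supply sunlight.
; Wood count caps water; running dry while below that cap pauses and shows Game Over.
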(event `self.ReceiveBeginPlay`
  (bind _returnvalue (`GameplayStatics.GetPlayerController` 0))
  (`|ExecutionSequence`
    (:`then_0`
      ;[1 1 1] Widget Creation
      (bind _returnvalue_2 (`|CreateWidget` "/Game/TOL/HUD/SunlightBar.SunlightBar_C"))
      (`UserWidget.AddToViewport` _returnvalue_2 0))
    (:`then_1`
      (bind _returnvalue_3 (`|CreateWidget` "/Game/TOL/HUD/NutrientBar.NutrientBar_C"))
      (`UserWidget.AddToViewport` _returnvalue_3 0))
    (:`then_2`
      (bind _returnvalue_4 (`|CreateWidget` "/Game/TOL/HUD/WaterBar.WaterBar_C"))
      (`UserWidget.AddToViewport` _returnvalue_4 0))
    (:`then_3`
      (bind _returnvalue_5 (`|CreateWidget` "/Game/TOL/HUD/ScrollBar.ScrollBar_C"))
      (`UserWidget.AddToViewport` _returnvalue_5 0))
    (:`then_4`
      (bind _returnvalue_6 (`|CreateWidget` "/Game/TOL/HUD/Tutorial.Tutorial_C"))
      (`UserWidget.AddToViewport` _returnvalue_6 0))
    (:`then_5`
      (bind _returnvalue_7 (`|CreateWidget` "/Game/TOL/HUD/Feedback.Feedback_C"))
      (`UserWidget.AddToViewport` _returnvalue_7 0))
    (:`then_6`
      (bind _returnvalue_8 (`|CreateWidget` "/Game/TOL/HUD/Mainmenu.Mainmenu_C"))
      (`UserWidget.AddToViewport` _returnvalue_8 0)
      ;[1 1 1] Menu inputs
      (`self.DisableInput` (`GameplayStatics.GetPlayerPawn` 0) _returnvalue)
      (set `PlayerController.bShowMouseCursor` true _returnvalue)
      (`GameplayStatics.SetGamePaused` true))
    (:`then_7`
      ;[1 1 1] Game music
      (`GameplayStatics.PlaySound2D` "/Game/TOL/Audio/Harmony.Harmony")
      (`GameplayStatics.PlaySound2D` "/Game/TOL/Audio/Harmony.Harmony")
      (`GameplayStatics.PlaySound2D` "/Game/TOL/Audio/Harmony.Harmony"))))

(event `self.ReceiveTick`
  (params (DeltaSeconds :type "Float (single-precision)"))
  ;[1 1 1] Resource Updating
  (`|ExecutionSequence`
    (:`then_0`
      (`self.Water System`))
    (:`then_1`
      (`self.Update Sunlight`))
    (:`then_2`
      (`self.Update Nutrients`))))

(fn `Update Nutrients`
  (if (<= (`self.CurrentNutrients`) (`KismetMathLibrary.Conv_IntToDouble` (`self.MaxNutrients`)))
    ;[1 1 1] Adding Nutrients/Root
    (set `self.CurrentNutrients` (+ (* (`self.Multiplier`) (* (`self.No.Roots`) (`GameplayStatics.GetWorldDeltaSeconds`))) (`self.CurrentNutrients`)))
    ;[1 1 1] Convert to percentage
    (set `self.NutrientPercentage` (/ (`self.CurrentNutrients`) (`KismetMathLibrary.Conv_IntToDouble` (`self.MaxNutrients`))))))

(fn `Update Sunlight`
  (if (<= (`self.CurrentSunlight`) (`self.MaxSunlight`))
    (set `self.CurrentSunlight` (+ (* (`self.Multiplier`) (* (`self.No. Leaves`) (`GameplayStatics.GetWorldDeltaSeconds`))) (`self.CurrentSunlight`)))
    (`|ExecutionSequence`
      (:`then_1`
        ;[1 1 1] Converting to percentage
        (set `self.SunlightPercentage` (/ (`self.CurrentSunlight`) (`self.MaxSunlight`)))))))

(fn `UserConstructionScript`)

(fn `Water System`
  (bind _returnvalue (`GameplayStatics.GetPlayerController` 0))
  ;[1 1 1] Setting max water
  (set `self.MaxWater` (* (`self.No.Wood`) 5))
  (if (< (`self.CurrentWater`) (`KismetMathLibrary.Conv_IntToDouble` (`self.MaxWater`)))
    (set `self.TreeFull` false)
    (set `self.CurrentWater` (+ (* (`self.Multiplier`) (- (* (`self.No.Roots`) (`GameplayStatics.GetWorldDeltaSeconds`)) (/ (* (`self.No. Leaves`) (`GameplayStatics.GetWorldDeltaSeconds`)) 2.0))) (`self.CurrentWater`)))
    (if true
      ;[1 1 1] Convert to percentage
      (set `self.Water Percentage` (/ (`self.CurrentWater`) (`KismetMathLibrary.Conv_IntToDouble` (`self.MaxWater`))))
      ;[1 1 1] Lose condition
      (if (<= (`self.CurrentWater`) 0.0)
        ;[1 1 1] Game Over
        (`GameplayStatics.SetGamePaused` true)
        (bind _returnvalue_2 (`|CreateWidget` "/Game/TOL/HUD/GameOver.GameOver_C"))
        (`UserWidget.AddToViewport` _returnvalue_2 0)
        (`self.DisableInput` (`GameplayStatics.GetPlayerPawn` 0) _returnvalue)
        (set `PlayerController.bShowMouseCursor` true _returnvalue)))
    (else
      (set `self.TreeFull` true))))