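; Player camera for a 2D tree-building game, stepping along a Y/Z tile grid to place or delete Wood, Leaf and Root blocks.
; Collider overlaps gate placement and drive feedback, with "Self" in component names marking occupied tiles.
; Wood and leaves require Z at or above zero, roots below, and each spends GM_2DGame sunlight and nutrients.
; Keys also cycle blocks, set the speed multiplier, toggle the tech tree and load TOLLevel.
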(event `InputAction|Left`
  (params (Key :type "Key Structure" :default "AnyKey"))
  ;[1 1 1] Movement
  (:`Pressed`
    (bind _output_get (set `self.Tile_Size` -16.0))
    (`self.K2_AddActorWorldOffset` (`KismetMathLibrary.MakeVector` 0.0 _output_get))
    (`self.Placing/Removing` :!label _label)))

(event `InputAction|Right`
  (params (Key :type "Key Structure" :default "AnyKey"))
  ;[1 1 1] Movement
  (:`Pressed`
    (bind _output_get (set `self.Tile_Size` 16.0))
    (`self.K2_AddActorWorldOffset` (`KismetMathLibrary.MakeVector` 0.0 _output_get))
    (goto _label)))

(event `InputAction|Down`
  (params (Key :type "Key Structure" :default "AnyKey"))
  ;[1 1 1] Movement
  (:`Pressed`
    (bind _output_get (set `self.Tile_Size` -16.0))
    (`self.K2_AddActorWorldOffset` (`KismetMathLibrary.MakeVector` 0.0 0.0 _output_get))
    (goto _label)))

(event `InputAction|Up`
  (params (Key :type "Key Structure" :default "AnyKey"))
  ;[1 1 1] Movement
  (:`Pressed`
    (bind _output_get (set `self.Tile_Size` 16.0))
    (`self.K2_AddActorWorldOffset` (`KismetMathLibrary.MakeVector` 0.0 0.0 _output_get))
    (goto _label)))

(event `Key|One`
  (params (Key :type "Key Structure" :default "AnyKey"))
  ;[1 1 1] Game speed adjustment
  (:`Pressed`
    (set `/Game/TOL/Blueprint/GM_2DGame.Multiplier` 1 (`self.2D GM`))))

(event `Key|Two`
  (params (Key :type "Key Structure" :default "AnyKey"))
  ;[1 1 1] Game speed adjustment
  (:`Pressed`
    (set `/Game/TOL/Blueprint/GM_2DGame.Multiplier` 2 (`self.2D GM`))))

(event `Key|Three`
  (params (Key :type "Key Structure" :default "AnyKey"))
  ;[1 1 1] Game speed adjustment
  (:`Pressed`
    (set `/Game/TOL/Blueprint/GM_2DGame.Multiplier` 3 (`self.2D GM`))))

(event `Key|Four`
  (params (Key :type "Key Structure" :default "AnyKey"))
  ;[1 1 1] Game speed adjustment
  (:`Pressed`
    (set `/Game/TOL/Blueprint/GM_2DGame.Multiplier` 3 (`self.2D GM`))))

(event `Key|R`
  (params (Key :type "Key Structure" :default "AnyKey"))
  ;[1 1 1] Cycling mechanic
  (:`Pressed`
    (switch `/Game/TOL/Blueprint/E_TileType` (`self.SelectedBlock`)
      (:`NewEnumerator0`
        (set `self.SelectedBlock` "NewEnumerator1"))
      (:`NewEnumerator1`
        (set `self.SelectedBlock` "NewEnumerator2"))
      (:`NewEnumerator2`
        (set `self.SelectedBlock` "NewEnumerator0")))))

(event `InputAction|Place`
  (params (Key :type "Key Structure" :default "AnyKey"))
  (bind _selectedblock (`self.SelectedBlock`))
  (bind _returnvalue (`SceneComponent.K2_GetComponentLocation` (`self.Collider`)))
  ;[1 1 1] Placing blocks
  (:`Pressed`
    ;;[1 1 1] Location is placable
    (if (`self.Can I Build Here?` _selectedblock)
      (switch `/Game/TOL/Blueprint/E_TileType` _selectedblock
        (:`NewEnumerator0`
          ;;[1 1 1] Spawn Wood
          (`self.Subtract Resources` 5.0 10.0
            (:`True`
              (`|SpawnActorFromClass` "/Game/TOL/Blueprint/BP_Wood.BP_Wood_C" (`KismetMathLibrary.MakeTransform` _returnvalue) "Undefined" "OverrideRootScale"))))
        (:`NewEnumerator1`
          ;;[1 1 1] Spawn Leaf
          (`self.Subtract Resources` 10.0 5.0
            (:`True`
              (`|SpawnActorFromClass` "/Game/TOL/Blueprint/BP_Leaf.BP_Leaf_C" (`KismetMathLibrary.MakeTransform` _returnvalue) "Undefined" "OverrideRootScale"))))
        (:`NewEnumerator2`
          ;;[1 1 1] Spwan Root
          (`self.Subtract Resources` 20.0 20.0
            (:`True`
              (`|SpawnActorFromClass` "/Game/TOL/Blueprint/BP_Root.BP_Root_C" (`KismetMathLibrary.MakeTransform` _returnvalue) "Undefined" "OverrideRootScale")))))
      (`self.Placing/Removing`))))

(event `InputAction|Delete`
  (params (Key :type "Key Structure" :default "AnyKey"))
  ;[1 1 1] Delete block
  (:`Pressed`
    (`self.Delete function`)
    (`self.Delete function`)
    (`self.Placing/Removing`)
    (`KismetSystemLibrary.Delay` 0.2)
    (`ActorComponent.Deactivate` (`self.ParticleSystem`))))

(event `Key|Escape`
  (params (Key :type "Key Structure" :default "AnyKey"))
  (:`Pressed`
    (`GameplayStatics.OpenLevel` "TOLLevel")))

(event `Key|I`
  (params (Key :type "Key Structure" :default "AnyKey"))
  (:`Pressed`
    (`KismetSystemLibrary.PrintString` (`|GetEnumeratorNameAsString` (`self.PlaceFeedback`)))))

(event `self.ReceiveBeginPlay`
  ;[1 1 1] Begin play
  (`|ExecutionSequence`
    (:`then_0`
      ;;[1 1 1] Set the value of game mode
      (set `self.2D GM` (cast `/Game/TOL/Blueprint/GM_2DGame` (`GameplayStatics.GetGameMode`) :!pure true))
      (`self.Placing/Removing`))
    (:`then_1`
      ;;[1 1 1] Stop the particle system from working at the stat of the game
      (`ActorComponent.Deactivate` (`self.ParticleSystem`)))
    (:`then_2`
      (bind _returnvalue (`|CreateWidget` "/Game/TOL/HUD/TechnologyTree.TechnologyTree_C"))
      (set `self.TechTreeHUD` _returnvalue))))

(event `InputAction|Open Tech Tree`
  (params (Key :type "Key Structure" :default "AnyKey"))
  (bind _returnvalue (`GameplayStatics.GetPlayerController` 0))
  (bind _techtreehud (`self.TechTreeHUD`))
  (:`Pressed`
    (`/Engine/EditorBlueprintResources/StandardMacros.FlipFlop`
      (:`A`
        (set `PlayerController.bShowMouseCursor` true _returnvalue)
        (`UserWidget.AddToViewport` _techtreehud 0))
      (:`B`
        (set `PlayerController.bShowMouseCursor` false _returnvalue)
        (`Widget.RemoveFromParent` _techtreehud)))))

(fn `Am I Above Ground?`
  (returns (Result :type Boolean))
  (bind (_returnvalue_x _returnvalue_y _returnvalue_z) (`KismetMathLibrary.BreakVector` (`self.K2_GetActorLocation`)))
  (return (>= _returnvalue_z 0.0)))

(fn `Can I Build Here?`
  (params (`Tile Type` :type "/Game/TOL/Blueprint/E_TileType Enum"))
  (returns (Result :type Boolean))
  (bind _inoverlappingcomponents (`PrimitiveComponent.GetOverlappingComponents` (`self.Collider`)))
  ;[1 1 1] if 0 then cannot place
  (if (== (`KismetArrayLibrary.Array_Length` _inoverlappingcomponents) 0)
    (return false)
    (else
      (for _array_element _inoverlappingcomponents
        ;[1 1 1] If a component has self in name then can place
        (if (`KismetStringLibrary.Contains` (`KismetSystemLibrary.GetDisplayName` _array_element) "Self")
          (return false)))
      (switch `/Game/TOL/Blueprint/E_TileType` `Tile Type`
        (:`NewEnumerator0`
          _)
        (:`NewEnumerator1`
          _)
        (:`NewEnumerator2`
          ;[1 1 1] If below ground then can place roots
          (return (not (`self.Am I Above Ground?`)))))
      ;[1 1 1] If above ground then can place wood and leaves
      (return (`self.Am I Above Ground?`)))))

(fn `Delete function`
  (bind _inoverlappingcomponents (`PrimitiveComponent.GetOverlappingComponents` (`self.Collider`)))
  (if (== (`KismetArrayLibrary.Array_Length` _inoverlappingcomponents) 0)
    (return)
    (else
      (for _array_element _inoverlappingcomponents
        ;[1 1 1] If a component has self in name then can delete
        (if (`KismetStringLibrary.Contains` (`KismetSystemLibrary.GetDisplayName` _array_element) "Self")
          ;[1 1 1] What happens when deleted
          (`self.K2_DestroyActor` (`ActorComponent.GetOwner` _array_element))
          (`ActorComponent.Activate` (`self.ParticleSystem`) false)
          (return)))
      (return))))

(fn `FollowMouse`
  (params (`Actor Reference` :type "Actor Object Reference") (`Tile Size` :type "Float (double-precision)")))

(fn `Placing/Removing`
  (bind _inoverlappingcomponents (`PrimitiveComponent.GetOverlappingComponents` (`self.Collider`)))
  (if (== (`KismetArrayLibrary.Array_Length` _inoverlappingcomponents) 0)
    (set `self.PlaceFeedback` "NewEnumerator2")
    (return)
    (else
      (for _array_element _inoverlappingcomponents
        ;[1 1 1] If component contains self than can be deleted
        (if (`KismetStringLibrary.Contains` (`KismetSystemLibrary.GetDisplayName` _array_element) "Self")
          (set `self.PlaceFeedback` "NewEnumerator1")
          (return)
          (else
            (set `self.PlaceFeedback` "NewEnumerator0" :!label _label)
            (return))))
      (goto _label))))

(fn `UserConstructionScript`)