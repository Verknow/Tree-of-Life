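; BP_Leaf is a 2D leaf actor that grows in and counts toward the game mode's leaf total.
; If more than one leaf exists, it plays a growth flipbook and sound, then finalizes after a fixed delay; otherwise it finalizes immediately.
; Tick separately fills a Construction widget progress bar using speed and multiplier, hiding it when full.
; Finalizing sets the grown sprite and increments the count; destruction decrements it.
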(event `self.ReceiveBeginPlay`
  (if (> (`/Game/TOL/Blueprint/GM_2DGame.No. Leaves` (cast `/Game/TOL/Blueprint/GM_2DGame` (`GameplayStatics.GetGameMode`) :!pure true)) 1)
    (`PaperFlipbookComponent.SetFlipbook` (`self.LeafGrow`) "/Game/TOL/Sprites/Leaf/Leaf/leafGrow.leafGrow")
    (`PaperFlipbookComponent.SetPlayRate` (`self.LeafGrow`) (`self.GrowthMultiplyer`))
    (`PaperFlipbookComponent.PlayFromStart` (`self.LeafGrow`))
    (`|ExecutionSequence`
      (:`then_0`
        (`GameplayStatics.PlaySound2D` "/Game/TOL/Audio/PlacingSound1.PlacingSound1") ; Sound effect
        (`PaperSpriteComponent.SetSprite` (`self.Leaf`) null)
        (`KismetSystemLibrary.Delay` 0.2))
      (:`then_1`
        (`KismetSystemLibrary.Delay` 12.0)
        (`PaperFlipbookComponent.SetFlipbook` (`self.LeafGrow`) null :!label _label)
        (`PaperSpriteComponent.SetSprite` (`self.Leaf`) "/Game/TOL/Sprites/LeafSprite3.LeafSprite3")
        (`ActorComponent.Deactivate` (`self.LeafBurst`))
        ;[1 1 1] +/- amount of leaves
        (`/Engine/EditorBlueprintResources/StandardMacros.IncrementInt` (`/Game/TOL/Blueprint/GM_2DGame.No. Leaves` (cast `/Game/TOL/Blueprint/GM_2DGame` (`GameplayStatics.GetGameMode`) :!pure true)))))
    (else
      (`PaperFlipbookComponent.SetFlipbook` (`self.LeafGrow`) null)
      (bind _asconstruction (cast `/Game/TOL/HUD/Construction` (`WidgetComponent.GetUserWidgetObject` (`self.GrowthBar`))))
      (`Widget.SetVisibility` _asconstruction "Hidden")
      (goto _label))))

(event `self.ReceiveTick`
  (params (DeltaSeconds :type "Float (single-precision)"))
  (bind _asconstruction (cast `/Game/TOL/HUD/Construction` (`WidgetComponent.GetUserWidgetObject` (`self.GrowthBar`))))
  (if (<= (`self.Growth`) 99.0)
    (`|ExecutionSequence`
      (:`then_0`
        (`ProgressBar.SetPercent` (`/Game/TOL/HUD/Construction.ProgressBar_24` _asconstruction) (/ (`self.Growth`) 100.0)))
      (:`then_1`
        (`self.Growing`)))
    (else
      (`Widget.SetVisibility` _asconstruction "Hidden"))))

(event `self.ReceiveDestroyed`
  ;[1 1 1] +/- amount of leaves
  (`/Engine/EditorBlueprintResources/StandardMacros.DecrementInt` (`/Game/TOL/Blueprint/GM_2DGame.No. Leaves` (cast `/Game/TOL/Blueprint/GM_2DGame` (`GameplayStatics.GetGameMode`) :!pure true))))

(fn `Growing`
  (set `self.Growth` (+ (* (* (`self.Growth speed`) (`self.GrowthMultiplyer`)) (`GameplayStatics.GetWorldDeltaSeconds`)) (`self.Growth`))))

(fn `UserConstructionScript`)